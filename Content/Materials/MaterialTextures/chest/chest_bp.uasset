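; Chest Blueprint that opens when the player uses the Key2 item on it.
; Looking at it updates the HUD with either a use prompt naming the held key or a hint to find the key.
; Interacting with Key2 held plays a timeline that rotates the lid component, then destroys the key.
; The CloseChest event is an empty stub.
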(event `Event Look At`
  (params (PlayerCharacter :type "/Game/FirstPersonBP/Blueprints/FPSCharacter Object Reference") (GameMode :type "/Game/FirstPersonBP/Blueprints/FirstPersonGameMode Object Reference"))
  (bind _hud (`/Game/FirstPersonBP/Blueprints/FPSCharacter.HUD` PlayerCharacter))
  (bind _currentlyhelditem (`/Game/FirstPersonBP/Blueprints/FPSCharacter.CurrentlyHeldItem` PlayerCharacter))
  (if (== _currentlyhelditem (`self.key 2`))
    (`/Game/UI/Heads_Up_Display.UpdateMessage` _hud (`|FormatText` "Press B to use {name}" (`/Game/Items/Item_Parent.ItemName` _currentlyhelditem)))
    (else
      (`/Game/UI/Heads_Up_Display.UpdateMessage` _hud "Find the Key to Open This Door"))))

(event `CustomEvent_1`
  (params (PlayerCharacter :type "/Game/FirstPersonBP/Blueprints/FPSCharacter Object Reference"))
  (bind _currentlyhelditem (`/Game/FirstPersonBP/Blueprints/FPSCharacter.CurrentlyHeldItem` PlayerCharacter))
  (if (== _currentlyhelditem (`self.key 2`))
    (`self.OpenChest`)
    (`self.K2_DestroyActor` _currentlyhelditem)))

(event `OpenChest`
  (bind (_direction _lidposition) (`Timeline|ChestOpening`)
    (:`Update`
      (`SceneComponent.K2_SetRelativeRotation` (`self.w`) (* (struct :`Pitch` -120.0) _lidposition) false false))))

(event `Close Chest`)

(fn `UserConstructionScript`)