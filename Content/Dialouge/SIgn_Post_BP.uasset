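; Sign post Blueprint that shows or hides a dialogue widget when its Interact event fires.
; If the stored widget is valid, Interact removes it from the viewport and clears the reference.
; Otherwise it creates a Dialouge_widget for player controller 0, adds it to the viewport and sets its DialougeText from the sign's MyText variable.
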(event `/Game/Dialouge/interact_i.interact`
  (`/Engine/EditorBlueprintResources/StandardMacros.IsValid` (`self.dialougeWidget`)
    (:`Is Valid`
      (`Widget.RemoveFromParent` (`self.dialougeWidget`))
      (set `self.dialougeWidget` null))
    (:`Is Not Valid`
      (bind _returnvalue (`|CreateWidget` "/Game/Dialouge/Dialouge_widget.Dialouge_widget_C" (`GameplayStatics.GetPlayerController` 0)))
      (bind _output_get (set `self.dialougeWidget` _returnvalue))
      (`UserWidget.AddToViewport` _output_get 0)
      (set `/Game/Dialouge/Dialouge_widget.Dialouge_Text` (`self.myText`) (`self.dialougeWidget`)))))

(fn `UserConstructionScript`)