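; Key pickup actor that grants the FPSCharacter a key, plays a sound at its location and destroys itself.
; Box overlap by the FPSCharacter caches the character, enables input and opens a Gate; end overlap reverses the input and Gate.
; The Interact axis event runs through that Gate without checking the axis value, so any firing while open collects the key.
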(event `InputAxis|Interact`
  (params (AxisValue :type "Float (single-precision)"))
  ;[1 1 1] open_drawer if close and has key
  (`/Engine/EditorBlueprintResources/StandardMacros.Gate` true :!label _label
    (:`Exit`
      (set `/Game/FirstPersonBP/Blueprints/FPSCharacter.has_key` true (stale `self.Box.OnComponentBeginOverlap` _asfpscharacter))
      (`GameplayStatics.PlaySoundAtLocation` "/Game/StarterContent/Audio/Light01_Cue.Light01_Cue" (`self.K2_GetActorLocation`) (struct) 1.0 1.0 0.0 null null null)
      (`self.K2_DestroyActor`))))

(event `self.Box.OnComponentBeginOverlap`
  (params (OverlappedComponent :type "PrimitiveComponent Object Reference") (OtherActor :type "Actor Object Reference") (OtherComp :type "PrimitiveComponent Object Reference") (OtherBodyIndex :type Integer) (bFromSweep :type Boolean) (SweepResult :type "HitResult Structure (by ref)"))
  ;[1 1 1] open_drawer if close and has key
  (bind _asfpscharacter (cast `/Game/FirstPersonBP/Blueprints/FPSCharacter` OtherActor))
  (`self.EnableInput` (`GameplayStatics.GetPlayerController` 0))
  (goto _label :!via `Open`))

(event `self.Box.OnComponentEndOverlap`
  (params (OverlappedComponent :type "PrimitiveComponent Object Reference") (OtherActor :type "Actor Object Reference") (OtherComp :type "PrimitiveComponent Object Reference") (OtherBodyIndex :type Integer))
  ;[1 1 1] open_drawer if close and has key
  (cast `/Game/FirstPersonBP/Blueprints/FPSCharacter` OtherActor)
  (`self.DisableInput` (`GameplayStatics.GetPlayerController` 0))
  (goto _label :!via `Close`))

(fn `UserConstructionScript`)