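; Locked drawer actor that slides open and closed when a nearby FPSCharacter holds the key.
; Box overlap caches the character and toggles input and a gate.
; The Interact axis event checks HasKey, then passes through the gate to a FlipFlop that plays or reverses a timeline, lerping the mesh's Y position with hard-coded X and Z.
; Without the key, the axis event plays an explosion sound at the drawer.
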(event `InputAxis|Interact`
  (params (AxisValue :type "Float (single-precision)"))
  ;[1 1 1] open_drawer if close and has key
  (if (`/Game/FirstPersonBP/Blueprints/FPSCharacter.has_key` (stale `self.Box.OnComponentBeginOverlap` _asfpscharacter))
    (`/Engine/EditorBlueprintResources/StandardMacros.Gate` true :!label _label
      (:`Exit`
        ;[1 1 1] open/closer drawer animation
        (`/Engine/EditorBlueprintResources/StandardMacros.FlipFlop`
          (:`A`
            (bind (_direction _drawer_track) (`Timeline|open/close drawer` :!label _label_2)
              (:`Update`
                (`SceneComponent.K2_SetRelativeLocationAndRotation` :`self` (`self.StaticMesh`) :`NewLocation` (`KismetMathLibrary.MakeVector` 440.0 (`KismetMathLibrary.Lerp` (`self.closed_pos`) (`self.open_pos`) _drawer_track) 4700.0)))))
          (:`B`
            (goto _label_2 :!via `Reverse`)))))
    (else
      (`GameplayStatics.PlaySoundAtLocation` "/Game/StarterContent/Audio/Explosion02.Explosion02" (`self.K2_GetActorLocation`) (struct) 1.0 1.0 0.0 null null null))))

(event `self.Box.OnComponentBeginOverlap`
  (params (OverlappedComponent :type "PrimitiveComponent Object Reference") (OtherActor :type "Actor Object Reference") (OtherComp :type "PrimitiveComponent Object Reference") (OtherBodyIndex :type Integer) (bFromSweep :type Boolean) (SweepResult :type "HitResult Structure (by ref)"))
  ;[1 1 1] open_drawer if close and has key
  (bind _asfpscharacter (cast `/Game/FirstPersonBP/Blueprints/FPSCharacter` OtherActor))
  (`self.EnableInput` (`GameplayStatics.GetPlayerController` 0))
  (goto _label :!via `Open`))

(event `self.Box.OnComponentEndOverlap`
  (params (OverlappedComponent :type "PrimitiveComponent Object Reference") (OtherActor :type "Actor Object Reference") (OtherComp :type "PrimitiveComponent Object Reference") (OtherBodyIndex :type Integer))
  ;[1 1 1] open_drawer if close and has key
  (cast `/Game/FirstPersonBP/Blueprints/FPSCharacter` OtherActor)
  (`self.DisableInput` (`GameplayStatics.GetPlayerController` 0))
  (goto _label :!via `Close`))

(fn `UserConstructionScript`)