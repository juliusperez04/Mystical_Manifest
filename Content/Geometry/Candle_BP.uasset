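; Candle Blueprint that pairs a mesh with a flickering point light and a particle effect, with an Enabled toggle.
; On BeginPlay, the Candle_Flicker timeline drives the light's intensity between configurable minimum and maximum values.
; SetEnabled shows or hides the light and particles, and turns off the mesh's shadow casting while lit.
; The construction script calls SetEnabled to apply the Enabled state.
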(event `self.ReceiveBeginPlay`
  (bind (_direction _intensity) (`Timeline|Candle_Flicker`)
    (:`Update`
      (`LightComponent.SetIntensity` (`self.PointLight`) (`KismetMathLibrary.Lerp` (`self.MinIntensity`) (`self.MaxIntensity`) _intensity)))))

(fn `SetEnabled`
  (params (Enabled :type Boolean))
  (bind _output_get (set `self.Enabled` Enabled))
  (`SceneComponent.SetVisibility` (`self.PointLight`) _output_get false)
  (`SceneComponent.SetVisibility` (`self.ParticleSystem`) _output_get false)
  (`PrimitiveComponent.SetCastShadow` (`self.StaticMesh`) (not _output_get)))

(fn `UserConstructionScript`
  (`self.SetEnabled` (`self.Enabled`)))